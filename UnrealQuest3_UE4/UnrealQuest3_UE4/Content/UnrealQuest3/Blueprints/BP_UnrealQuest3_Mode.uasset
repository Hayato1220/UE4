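; Game mode Blueprint for UnrealQuest3 that handles level transitions and background music.
; JumpToNextLevel takes a level and a sound cue, and swaps the Audio component to that cue with a short fade-in only when it differs from the current track.
; It also starts a one-shot timer that opens the requested level by object reference after a five-second delay.
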(event `JumpToNextLevel`
  (params (Level :type "World Soft Object Reference") (`sound cue` :type "SoundCue Object Reference"))
  (`|ExecutionSequence`
    (:`then_0`
      (if (!= `sound cue` (`self.CurentBGM`))
        (`AudioComponent.Stop` (`self.Audio`))
        (bind _output_get (set `self.CurentBGM` `sound cue`))
        (`AudioComponent.SetSound` (`self.Audio`) _output_get)
        (`AudioComponent.FadeIn` (`self.Audio`) 1.0 1.0 0.0 "Linear")))
    (:`then_1`
      (`KismetSystemLibrary.K2_SetTimerDelegate` (delegate `OpenLevel`) 5.0))))

(event `OpenLevel`
  (`GameplayStatics.OpenLevelBySoftObjectPtr` (stale `JumpToNextLevel` Level)))

(fn `UserConstructionScript`)