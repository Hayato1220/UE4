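; BP_Target is a moving target actor that is destroyed when it takes any damage.
; Movement comes from an InterpToMovement component that travels along control points.
; The construction script copies the actor's Duration, BehaviourType and ControlPoints variables into that component, so each instance can have its own path, timing and movement behaviour.
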(event `self.ReceiveAnyDamage`
  (params (Damage :type "Float (single-precision)") (DamageType :type "DamageType Object Reference") (InstigatedBy :type "Controller Object Reference") (DamageCauser :type "Actor Object Reference"))
  (`self.K2_DestroyActor`))

(fn `UserConstructionScript`
  (set `InterpToMovementComponent.Duration` (`self.Duration`) (`self.InterpToMovement`))
  (set `InterpToMovementComponent.BehaviourType` (`self.Behaviour Type`) (`self.InterpToMovement`))
  (set `InterpToMovementComponent.ControlPoints` (`self.Control Points`) (`self.InterpToMovement`)))